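; Base gameplay ability Blueprint that provides player lookup and triggers cooldown display on the owning player's UI.
; GetPlayerInfo casts the owning actor to CaptureCharacter and its controller to BP_CaptureController.
; The CL_DoUICooldown event calls DoUICooldown, which exits on the server, then starts cooldown on each UIPrimary slot whose ability class matches this one.
; ActivateAbility and OnEndAbility are empty, disabled stubs.
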(event `CL_DoUICooldown`
  (`self.DoUICooldown`))

(fn `DoUICooldown`
  (bind (_capturecharacter _capturecontroller) (`self.GetPlayerInfo`))
  (if (`KismetSystemLibrary.IsServer`)
    (return)
    (else
      (bind _uiprimary (`/Game/_MainGameStuff/Blueprints_CaptureGame/Game/BP_CaptureController.UIPrimary` _capturecontroller))
      (`/Engine/EditorBlueprintResources/StandardMacros.IsValid` _uiprimary
        (:`Is Valid`
          (for _array_element (`/Game/_MainGameStuff/UI/UI_Primary.Slots` _uiprimary)
            (bind _returnvalue (`self.GetAbilityInfo`))
            (bind (_abilityinfo_cooldownduration _abilityinfo_cost _abilityinfo_costtype _abilityinfo_uimat _abilityinfo_abilityclass) (break `GameplayAbilityInfo` (`/Game/_MainGameStuff/UI/UI_AbilitySlot.AbilityInfo` _array_element)))
            (if (== _abilityinfo_abilityclass (`.AbilityClass` (break `GameplayAbilityInfo` _returnvalue)))
              (`/Game/_MainGameStuff/UI/UI_AbilitySlot.StartCooldown` _array_element))))
        (:`Is Not Valid`
          (`KismetSystemLibrary.PrintString` "UI Primary not valid in DO UICooldown function"))))))

(fn `GetPlayerInfo`
  (returns (CaptureCharacter :type "/Game/_MainGameStuff/Blueprints_CaptureGame/Game/CaptureCharacter Object Reference") (CaptureController :type "/Game/_MainGameStuff/Blueprints_CaptureGame/Game/BP_CaptureController Object Reference"))
  (bind _ascapture_character (cast `/Game/_MainGameStuff/Blueprints_CaptureGame/Game/CaptureCharacter` (`self.GetOwningActorFromActorInfo`) :!pure true))
  (return _ascapture_character (cast `/Game/_MainGameStuff/Blueprints_CaptureGame/Game/BP_CaptureController` (`Pawn.GetController` _ascapture_character) :!pure true)))