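; Explosion actor for the Fireball ability that applies the fireball gameplay effect and knockback to nearby characters.
; On BeginPlay, only on the authority, it runs a small sphere overlap at its particle system's location and keeps the CaptureCharacter hits.
; Each hit receives Effect_Fireball through its own Ability System Component and is launched away from the blast center with an added upward bias.
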(event `self.ReceiveBeginPlay`
  (`/Engine/EditorBlueprintResources/ActorMacros.Switch Has Authority`
    (:`Authority`
      (bind _outactors (`KismetSystemLibrary.SphereOverlapActors` (`SceneComponent.K2_GetComponentLocation` (`self.ParticleSystem`)) 60.0 (`|MakeArray` "ObjectTypeQuery3" "ObjectTypeQuery4" :!type "EObjectTypeQuery Enum")))
      (for _array_element _outactors
        (bind _ascapture_character (cast `/Game/_MainGameStuff/Blueprints_CaptureGame/Game/CaptureCharacter` _array_element))
        (bind _output_get (set `self.PlayersHit` _ascapture_character))
        (`AbilitySystemComponent.BP_ApplyGameplayEffectToSelf` :`self` (`AbilitySystemBlueprintLibrary.GetAbilitySystemComponent` _output_get) :`GameplayEffectClass` "/Game/_MainGameStuff/GameplayAbilities/Fireball/Effect_Fireball.Effect_Fireball_C")
        (`Character.LaunchCharacter` _output_get (* (`KismetMathLibrary.MakeVector` (.x (`KismetMathLibrary.GetDirectionUnitVector` (`SceneComponent.K2_GetComponentLocation` (`self.ParticleSystem`)) (`SceneComponent.K2_GetComponentLocation` (`Character.CapsuleComponent` (`self.PlayersHit`))))) (.y (`KismetMathLibrary.GetDirectionUnitVector` (`SceneComponent.K2_GetComponentLocation` (`self.ParticleSystem`)) (`SceneComponent.K2_GetComponentLocation` (`Character.CapsuleComponent` (`self.PlayersHit`))))) (+ (.z (`KismetMathLibrary.GetDirectionUnitVector` (`SceneComponent.K2_GetComponentLocation` (`self.ParticleSystem`)) (`SceneComponent.K2_GetComponentLocation` (`Character.CapsuleComponent` (`self.PlayersHit`))))) 1.0)) 300.0) false false)))))

(fn `UserConstructionScript`)