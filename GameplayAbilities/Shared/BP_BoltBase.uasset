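; BP_BoltBase is a bolt projectile base for gameplay abilities that applies a Gameplay Effect to characters it hits.
; On server authority, collision overlaps ignore the instigator and already-hit actors, then apply BoltEffect through a CaptureCharacter's Ability System Component.
; After applying it or hitting any non-character actor, the bolt disables collision, hides and destroys itself after a short delay.
; A timeout from projectile movement activation also destroys it.
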(event `self.BoltCollision.OnComponentBeginOverlap`
  (params (OverlappedComponent :type "PrimitiveComponent Object Reference") (OtherActor :type "Actor Object Reference") (OtherComp :type "PrimitiveComponent Object Reference") (OtherBodyIndex :type Integer) (bFromSweep :type Boolean) (SweepResult :type "HitResult Structure (by ref)"))
  (bind _hitactor (`self.HitActor`))
  (`/Engine/EditorBlueprintResources/ActorMacros.Switch Has Authority`
    (:`Authority`
      (if (!= OtherActor (`self.GetInstigator`))
        (if (not (`KismetArrayLibrary.Array_Contains` _hitactor OtherActor))
          (bind _returnvalue (`KismetArrayLibrary.Array_Add` _hitactor OtherActor))
          (bind _output_get (set `self.ActorHit` _returnvalue))
          (bind _output (`|GetArrayItem` (`self.HitActor`) _output_get))
          (`KismetSystemLibrary.PrintString` (`KismetSystemLibrary.GetDisplayName` _output))
          (bind (_ascapture_character _bsuccess) (cast `/Game/_MainGameStuff/Blueprints_CaptureGame/Game/CaptureCharacter` _output :!pure true))
          (if _bsuccess
            (bind _returnvalue_2 (`AbilitySystemBlueprintLibrary.GetAbilitySystemComponent` _ascapture_character))
            (`/Engine/EditorBlueprintResources/StandardMacros.IsValid` _returnvalue_2
              (:`Is Valid`
                (`AbilitySystemComponent.BP_ApplyGameplayEffectToSelf` :`self` _returnvalue_2 :`GameplayEffectClass` (`self.BoltEffect`))
                (`PrimitiveComponent.SetCollisionEnabled` (`self.BoltCollision`) "NoCollision")
                (`self.SetActorHiddenInGame` self true)
                (`KismetSystemLibrary.Delay` 1.0)
                (`self.K2_DestroyActor`)))
            (else
              (`PrimitiveComponent.SetCollisionEnabled` (`self.BoltCollision`) "NoCollision")
              (`self.SetActorHiddenInGame` self true)
              (`KismetSystemLibrary.Delay` 1.0)
              (`self.K2_DestroyActor`))))))))

(event `self.ProjectileMovement.OnComponentActivated`
  (params (Component :type "ActorComponent Object Reference") (bReset :type Boolean))
  (`KismetSystemLibrary.Delay` 3.0)
  (`KismetSystemLibrary.PrintString` "Destroying...")
  (`self.K2_DestroyActor`))

(fn `UserConstructionScript`)