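; Player controller for a team-based capture game: starts on a viewing pawn, shows team selection, then requests spawns from the game mode.
; Initialize caches the possessed character and builds the local HUD, fed by health, mana and stamina updates.
; Input drives sprint, menu, chat, hotbar slots and attacks, with ranged cooldowns read from UI slots.
; Sprint, death and respawn switch on authority and forward to the server; a PlayerIsDead RepNotify triggers the death screen.
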(event `self.ReceiveBeginPlay`
  ;[1 1 1 1 36] Begin Play
  (`|ExecutionSequence`
    (:`then_1`
      (`/Engine/EditorBlueprintResources/ActorMacros.Switch Has Authority`
        (:`Authority`
          (bind _outactors (`GameplayStatics.GetAllActorsOfClass` "/Game/_MainGameStuff/Blueprints_CaptureGame/Game/StartingView.StartingView_C"))
          (`self.Possess` (`|GetArrayItem` _outactors)))))
    (:`then_2`
      (if (`self.IsLocalController`)
        (bind _returnvalue (`|CreateWidget` "/Game/_MainGameStuff/UMG/MyTeamSelection.MyTeamSelection_C" self))
        (`UserWidget.AddToViewport` _returnvalue 0)
        (set `self.bShowMouseCursor` true)))))

(event `self.AddAbilityToUI`
  (params (AbilityInfo :type "GameplayAbilityInfo Structure"))
  ;[1 1 1 1 36] Begin Play
  (if (not (`KismetSystemLibrary.IsServer`))
    (`/Game/_MainGameStuff/UI/UI_Primary.AddAbilityToSlots` (`self.UIPrimary`) AbilityInfo)))

(event `TeamSelected`
  (params (Team :type "/Game/_MainGameStuff/Blueprints_CaptureGame/Game/Teams Enum" :default "NewEnumerator0") (Class :type "/Game/_MainGameStuff/Blueprints_CaptureGame/Game/CaptureCharacter Class Reference") (TeamNumber :type Integer))
  ;[1 1 1] Spawn player on team
  (bind _output_get (set `self.SelectedTeam` Team))
  (bind _output_get_2 (set `self.SelectedClass` Class))
  (set `self.TeamNumber` TeamNumber)
  (`/Game/_MainGameStuff/Blueprints_CaptureGame/Game/BP_CaptureGamemode.RequestSpawn` (cast `/Game/_MainGameStuff/Blueprints_CaptureGame/Game/BP_CaptureGamemode` (`GameplayStatics.GetGameMode`) :!pure true) _output_get self _output_get_2))

(event `CL_Initialize`
  ;[1 1 1] Initializes and spawns the player with the correct abilities
  (if (`self.IsLocalPlayerController`)
    (`KismetSystemLibrary.Delay` 0.25 :!label _label)
    (`self.Initialize`)))

(event `SRV_Initialize`
  ;[1 1 1] Initializes and spawns the player with the correct abilities
  (if (`self.IsLocalPlayerController`)
    (goto _label)
    (else
      (`self.CL_Initialize`)
      (goto _label))))

(event `GetChatMessage`
  (params (TextToSend :type Text))
  ;[1 1 1] Get chat messages and update screen
  (bind _output_get (set `self.SenderText` TextToSend))
  (`self.UpdateChat` "" _output_get))

(event `UpdateChat`
  (params (SenderName :type Text) (SenderText :type Text))
  ;[1 1 1] Get chat messages and update screen
  (`/Game/_MainGameStuff/Blueprints_CaptureGame/Game/CaptureCharacter.UpdateChatBubble` (`self.CaptureCharacter`) SenderText))

(event `CL_UpdateManaOnPlayerScreen`
  (params (Mana :type "Float (double-precision)") (MaxMana :type "Float (double-precision)"))
  ;[1 1 1] Updates player mana on the UI
  (set `self.Mana` Mana)
  (set `self.MaxMana` MaxMana)
  (`/Game/_MainGameStuff/UI/UI_Glassball.SetPercentage` (`/Game/_MainGameStuff/UI/UI_Primary.Mana_Bar` (`self.UIPrimary`)) (/ (`self.Mana`) (`self.MaxMana`))))

(event `CL_UpdateStaminaOnPlayerScreen`
  (params (Stamina :type "Float (double-precision)") (MaxStamina :type "Float (double-precision)"))
  ;[1 1 1] Updates player stamina on the UI
  (set `self.Stamina` Stamina)
  (set `self.MaxStamina` MaxStamina)
  (`/Game/_MainGameStuff/UI/UI_Glassball.SetPercentage` (`/Game/_MainGameStuff/UI/UI_Primary.Stamina_Bar` (`self.UIPrimary`)) (/ (`self.Stamina`) (`self.MaxStamina`)))
  (if (<= (`self.Stamina`) 0.0)
    (`self.ToggleSprint` false) ; Ifstamina is empty, turn of Sprint state
  ))

(event `CL_UpdateHealthOnPlayerScreen`
  (params (Health :type "Float (double-precision)") (MaxHealth :type "Float (double-precision)"))
  (bind _returnvalue (/ Health MaxHealth))
  ;[1 1 1] Updates player health and kills the player if HP drops below 0
  (`/Game/_MainGameStuff/UI/UI_Glassball.SetPercentage` (`/Game/_MainGameStuff/UI/UI_Primary.Health_Bar` (`self.UIPrimary`)) _returnvalue)
  (if (<= _returnvalue 0.0)
    (`self.SetDeath`)))

(event `ToggleSprint`
  (params (State :type Boolean))
  ;[1 1 1] Activates the sprinting speed when shift is held down
  (`self.SprintSwitch` State))

(event `SetDeath`
  ;[1 1 1] Sets the Death Notify to kill the player
  (`self.DeathSwitch` :!label _label_2))

(event `SRV_ToggleSprint`
  (params (State :type Boolean))
  ;[1 1 1] Activates the sprinting speed when shift is held down
  (`self.SprintSwitch` State))

(event `SRV_SetDeath`
  (goto _label_2))

(event `SetViewAngles`
  (params (Reset :type Boolean) (YMin :type "Float (double-precision)") (YMax :type "Float (double-precision)"))
  ;[0.9974 0.1441 1] TODO: Sets different angles when the player is sprinting/walking
  (if Reset
    _))

(event `PlayerDeath`
  ;[1 1 1] Hides the Primary UI and brings up the death screen to allow player to respawn
  (if (`self.IsLocalPlayerController`)
    (`Widget.RemoveFromParent` (`self.UIPrimary`))
    (`self.UnPossess`)
    (`KismetSystemLibrary.Delay` 5.0)
    (bind _returnvalue (`|CreateWidget` "/Game/_MainGameStuff/UI/UI_Dead.UI_Dead_C" self)) ; Create the in-game menu widget.
    (bind _output_get (set `self.UIDead` _returnvalue))
    (`UserWidget.AddToViewport` _output_get 0)))

(event `PlayerRespawn`
  ;[1 1 1] Player Respawn Switch
  (`self.RespawnSwitch` :!label _label_3))

(event `SRV_PlayerRespawn`
  (goto _label_3))

(event `InputAction|Jump`
  (params (Key :type "Key Structure")))

(event `InputAxis|LookingRight`
  (params (AxisValue :type "Float (single-precision)")))

(event `InputAxis|LookingUp`
  (params (AxisValue :type "Float (single-precision)")))

(event `InputAxis|MoveForward`
  (params (AxisValue :type "Float (single-precision)")))

(event `InputAxis|MoveRight`
  (params (AxisValue :type "Float (single-precision)")))

(event `InputAction|Sprint`
  (params (Key :type "Key Structure"))
  (:`Pressed`
    ;[1 1 1] Activate Sprint Stamina Drain
    (if (`self.bCanMove`)
      (if (>= (`self.Stamina`) 25.0)
        (set `self.bIsSprinting` true)
        (`self.ToggleSprint` true)
        (`KismetSystemLibrary.Delay` 0.5)
        (if (not (`self.IsInputKeyDown` Key))
          (`self.ToggleSprint` false)))))
  (:`Released`
    (if (`self.bCanMove`)
      (set `self.bIsSprinting` false)
      (`self.ToggleSprint` false))))

(event `InputAction|Chat`
  (params (Key :type "Key Structure"))
  (bind _chatentry (`/Game/_MainGameStuff/UMG/ChatWindow.ChatEntry` (`/Game/_MainGameStuff/UI/UI_Primary.ChatBox` (`self.UIPrimary`))))
  (:`Pressed`
    ;[1 1 1] Allows player to chat and post to the chat window and bubbles
    (`Widget.SetUserFocus` _chatentry self)
    (`Widget.SetKeyboardFocus` _chatentry)
    (set `self.bShowMouseCursor` false)))

(event `InputAction|Toggle In-Game Menu`
  (params (Key :type "Key Structure"))
  (:`Pressed`
    ;[1 1 1] Toggles In-Game Menu
    (if (`self.inMenu?`)
      (set `self.inMenu?` false)
      (set `self.bCanMove` true)
      (`Widget.RemoveFromParent` (`self.GameMenu`))
      (`WidgetBlueprintLibrary.SetInputMode_GameOnly` self) ; Set input mode to game only.
      (else
        (set `self.inMenu?` true)
        (set `self.bCanMove` false)
        (bind _returnvalue (`|CreateWidget` "/Game/_MainGameStuff/UMG/IngameMenu.IngameMenu_C" self)) ; Create the in-game menu widget.
        (bind _output_get (set `self.GameMenu` _returnvalue))
        (`UserWidget.AddToViewport` _output_get 0)
        (`WidgetBlueprintLibrary.SetInputMode_GameAndUIEx` self (`self.GameMenu`) "LockAlways")))))

(event `InputAction|AttackWithSelectedAbility`
  (params (Key :type "Key Structure"))
  (bind _capturecharacter (`self.CaptureCharacter`))
  (bind _capturecharacter_2 (`self.CaptureCharacter`))
  (bind _israngedattacker_ (`/Game/_MainGameStuff/Blueprints_CaptureGame/Game/CaptureCharacter.IsRangedAttacker?` _capturecharacter))
  (:`Pressed`
    ;[1 1 1] Default Attack
    (if (not (`self.PlayerIsDead`))
      (`/Engine/EditorBlueprintResources/StandardMacros.IsValid` _capturecharacter
        (:`Is Valid`
          (if _israngedattacker_
            (if (not (`/Game/_MainGameStuff/Blueprints_CaptureGame/Game/CaptureCharacter.IsAbilityCharging?` (`self.CaptureCharacter`)))
              (`self.CheckForCooldown` (`self.SRV_AbilitySlot`)))
            (elif (`/Game/_MainGameStuff/Blueprints_CaptureGame/Game/CaptureCharacter.IsAttacking?` _capturecharacter_2)
              _
              (elif (> (`self.Stamina`) 5.0)
                (`/Game/_MainGameStuff/Blueprints_CaptureGame/Game/CaptureCharacter.SRV_DoMeleeAbility` _capturecharacter_2))))))))
  (:`Released`
    (if (not (`self.PlayerIsDead`))
      (`/Engine/EditorBlueprintResources/StandardMacros.IsValid` _capturecharacter
        (:`Is Valid`
          (if _israngedattacker_
            (`/Game/_MainGameStuff/Blueprints_CaptureGame/Game/CaptureCharacter.SRV_ReleaseRangeAbility` (`self.CaptureCharacter`))))))))

(event `SRV_SetSlot1`
  ;[1 1 1] Activates Abilities in the hot bar for their slot number
  (bind _output_get (set `self.SRV_AbilitySlot` 0))
  (`self.SRV_SetSlot` _output_get))

(event `InputAction|Slot1`
  (params (Key :type "Key Structure"))
  (:`Pressed`
    ;[1 1 1] Activates Abilities in the hot bar for their slot number
    (`self.SRV_SetSlot1`)))

(event `SRV_SetSlot2`
  ;[1 1 1] Activates Abilities in the hot bar for their slot number
  (bind _output_get (set `self.SRV_AbilitySlot` 1))
  (`self.SRV_SetSlot` _output_get))

(event `InputAction|Slot2`
  (params (Key :type "Key Structure"))
  (:`Pressed`
    ;[1 1 1] Activates Abilities in the hot bar for their slot number
    (`self.SRV_SetSlot2`)))

(event `SRV_SetSlot`
  (params (AbilitySlot :type Integer))
  (bind _capturecharacter (`self.CaptureCharacter`))
  ;[1 1 1] Activates Abilities in the hot bar for their slot number
  (bind _output_get (set `self.SRV_AbilitySlot` AbilitySlot))
  (set `/Game/_MainGameStuff/Blueprints_CaptureGame/Game/CaptureCharacter.CurrentSelectedAbility` (`|GetArrayItem` (`/Game/_MainGameStuff/Blueprints_CaptureGame/Game/CaptureCharacter.InitialAbilities` _capturecharacter) _output_get) _capturecharacter))

(event `Key|Gamepad_RightShoulder`
  (params (Key :type "Key Structure")))

(event `InputAction|Slot3`
  (params (Key :type "Key Structure"))
  (:`Pressed`
    ;[1 1 1] Activates Abilities in the hot bar for their slot number
    (`self.SRV_SetSlot3`)))

(event `SRV_SetSlot3`
  ;[1 1 1] Activates Abilities in the hot bar for their slot number
  (bind _output_get (set `self.SRV_AbilitySlot` 2))
  (`self.SRV_SetSlot` _output_get))

(event `SRV_SetSlot4`
  ;[1 1 1] Activates Abilities in the hot bar for their slot number
  (bind _output_get (set `self.SRV_AbilitySlot` 3))
  (`self.SRV_SetSlot` _output_get))

(event `InputAction|Slot4`
  (params (Key :type "Key Structure"))
  (:`Pressed`
    ;[1 1 1] Activates Abilities in the hot bar for their slot number
    (`self.SRV_SetSlot4`)))

(event `SRV_SetSlot5`
  ;[1 1 1] Activates Abilities in the hot bar for their slot number
  (bind _output_get (set `self.SRV_AbilitySlot` 4))
  (`self.SRV_SetSlot` _output_get))

(event `InputAction|Slot5`
  (params (Key :type "Key Structure"))
  (:`Pressed`
    ;[1 1 1] Activates Abilities in the hot bar for their slot number
    (`self.SRV_SetSlot5`)))

(event `CheckForCooldown`
  (params (AbilitySlot :type Integer))
  (bind _uiprimary (`self.UIPrimary`))
  (switch `int` AbilitySlot
    (:`0`
      (if (not (`/Game/_MainGameStuff/UI/UI_AbilitySlot.OnCooldown` (`/Game/_MainGameStuff/UI/UI_Primary.AbilitySlot1` _uiprimary)))
        (`self.SRV_CanDoAbility` :!label _label)))
    (:`1`
      (if (not (`/Game/_MainGameStuff/UI/UI_AbilitySlot.OnCooldown` (`/Game/_MainGameStuff/UI/UI_Primary.AbilitySlot2` _uiprimary)))
        (goto _label)))
    (:`2`
      (if (not (`/Game/_MainGameStuff/UI/UI_AbilitySlot.OnCooldown` (`/Game/_MainGameStuff/UI/UI_Primary.AbilitySlot3` _uiprimary)))
        (goto _label)))
    (:`3`
      (if (not (`/Game/_MainGameStuff/UI/UI_AbilitySlot.OnCooldown` (`/Game/_MainGameStuff/UI/UI_Primary.AbilitySlot4` _uiprimary)))
        (goto _label)))
    (:`4`
      (if (not (`/Game/_MainGameStuff/UI/UI_AbilitySlot.OnCooldown` (`/Game/_MainGameStuff/UI/UI_Primary.AbilitySlot5` _uiprimary)))
        (goto _label)))))

(event `SRV_CanDoAbility`
  ;[1 1 1] A simple ability switch
  (`/Game/_MainGameStuff/Blueprints_CaptureGame/Game/CaptureCharacter.SRV_StartRangeAbilityAnims` (`self.CaptureCharacter`)))

(fn `DeathSwitch`
  (if (`self.PlayerIsDead`)
    (return)
    (else
      (`/Engine/EditorBlueprintResources/ActorMacros.Switch Has Authority` ; Does the controller calling this have authority?
        (:`Authority`
          (set `self.PlayerIsDead` true) ; Setting the notify state
          (return))
        (:`Remote`
          (`self.SRV_SetDeath`) ; Call this again on the server.
          (return))))))

(fn `DisableMovement`
  (`self.SetIgnoreLookInput` true) ; Ignore player look input.
  (`self.SetIgnoreMoveInput` true) ; Ignore player move input.
  (set `self.bEnableMouseOverEvents` true)
  (set `self.bEnableClickEvents` true)
  (set `self.bShowMouseCursor` true)
  (set `self.bCanMove` false)
  (return))

(fn `EnableMovement`
  (`self.SetIgnoreLookInput` false) ; Stop ignoring player look input.
  (`self.SetIgnoreMoveInput` false) ; Stop ignoring player move input.
  (set `self.bEnableMouseOverEvents` false) ; Disable mouse over events.
  (set `self.bEnableClickEvents` false) ; Disable click events.
  (set `self.bShowMouseCursor` false) ; Hide the mouse cursor.
  (set `self.bCanMove` true)
  (return))

(fn `Initialize`
  (bind _ascharacter_base (cast `CharacterBase` (`self.K2_GetPawn`))
    (:`then`
      (bind _output_get (set `self.MyCharacterBase` _ascharacter_base))
      (bind _ascapture_character (cast `/Game/_MainGameStuff/Blueprints_CaptureGame/Game/CaptureCharacter` _output_get)
        (:`then`
          (bind _output_get_2 (set `self.CaptureCharacter` _ascapture_character))
          (set `/Game/_MainGameStuff/Blueprints_CaptureGame/Game/CaptureCharacter.TeamNumber` (`self.TeamNumber`) _output_get_2)
          (if (`self.IsLocalController` self)
            (bind _returnvalue (`|CreateWidget` "/Game/_MainGameStuff/UI/UI_Primary.UI_Primary_C" self))
            (bind _output_get_3 (set `self.UIPrimary` _returnvalue))
            (`UserWidget.AddToViewport` _output_get_3 0)
            (set `self.bCanMove` true)
            (set `self.bShowMouseCursor` false)
            (`WidgetBlueprintLibrary.SetInputMode_GameOnly` self)
            (set `self.Stamina` (`/Game/_MainGameStuff/Blueprints_CaptureGame/Game/CaptureCharacter.Stamina` (`self.CaptureCharacter`)))))
        (:`CastFailed`
          (`KismetSystemLibrary.PrintString` "Cast to CaptureCharacter from Controller failed"))))
    (:`CastFailed`
      (`KismetSystemLibrary.PrintString` "Cast to CharacterBase from Controller failed"))))

(fn `OnRep_PlayerIsDead`
  (if (`self.PlayerIsDead`)
    (message `/Game/_MainGameStuff/Blueprints_CaptureGame/Interfaces/BPI_CaptureCharacter.SetCharacterDeath` (`self.CaptureCharacter`) (`self.PlayerIsDead`)) ; Parse death state to player character.
    (`self.DisableMovement`) ; Disable movement on dead player's end.
    (`self.PlayerDeath`) ; Kill the player.
    (return)))

(fn `Respawn`
  (`/Engine/EditorBlueprintResources/ActorMacros.Switch Has Authority` ; Ensure only server can run the respawn.
    (:`Authority`
      (`self.UnPossess`)
      (`self.TeamSelected` (`self.SelectedTeam`) (`self.SelectedClass`)))
    (:`Remote`
      (return))))

(fn `RespawnSwitch`
  (if (`self.PlayerIsDead`)
    (`/Engine/EditorBlueprintResources/ActorMacros.Switch Has Authority` ; Does the controller calling this have authority?
      (:`Authority`
        (set `self.PlayerIsDead` false) ; Trigger respawn w/notify on bool change
        (`self.Respawn`)
        (return))
      (:`Remote`
        (`Widget.RemoveFromParent` (`self.UIDead`))
        (`self.SRV_PlayerRespawn`) ; Run this again on the server.
      ))
    (else
      (return))))

(fn `SprintSwitch`
  (params (State :type Boolean))
  (locals (SprintState :type Boolean))
  (bind _capturecharacter (`self.CaptureCharacter`))
  (bind _output_get (set `local.SprintState` State)) ; Stored for local use
  (if (== _output_get (`self.IsSprintingStateCheck`))
    (return)
    (else
      (`/Engine/EditorBlueprintResources/ActorMacros.Switch Has Authority` ; Does the player have authority?
        (:`Authority`
          (set `self.IsSprintingStateCheck` (`local.SprintState`))
          (if (`local.SprintState`)
            (`self.UpdatePlayerSpeed` (`self.SprintSpeed`)) ; Set character speed to sprint speed.
            (`self.UpdateViewAngles` false (`self.SprintViewRange`))
            (`/Game/_MainGameStuff/Blueprints_CaptureGame/Game/CaptureCharacter.StaminaDrainON` _capturecharacter)
            (return)
            (else
              (`self.UpdatePlayerSpeed` (`self.WalkSpeed`)) ; Set character speed to walk speed.
              (`self.UpdateViewAngles` true)
              (`/Game/_MainGameStuff/Blueprints_CaptureGame/Game/CaptureCharacter.StaminaDrainOFF` _capturecharacter)
              (return))))
        (:`Remote`
          (`self.SRV_ToggleSprint` (`local.SprintState`)) ; Run this again on the server.
          (if (`local.SprintState`)
            (`self.UpdatePlayerSpeed` (`self.SprintSpeed`)) ; Set character speed to sprint speed.
            (else
              (`self.UpdatePlayerSpeed` (`self.WalkSpeed`)) ; Set character speed to walk speed.
            ))
          (return))))))

(fn `TryActivateAbilityInSlot`
  (params (SlotNumber :type Integer))
  (bind (_abilityclass _valid) (`/Game/_MainGameStuff/UI/UI_Primary.GetSlotAbilityClass` (`self.UIPrimary`) SlotNumber))
  (if _valid
    (set `/Game/_MainGameStuff/Blueprints_CaptureGame/Game/CaptureCharacter.CurrentSelectedAbility` _abilityclass (`self.CaptureCharacter`))
    (else
      (`KismetSystemLibrary.PrintString` "Slot Ability Class not valid in the CaptureController"))))

(fn `UserConstructionScript`)